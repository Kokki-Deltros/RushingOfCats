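; Spike trap that repeatedly moves its mesh vertically and kills BP_IA_Player actors in its box while lethal.
; A timeline with adjustable play rate lerps the mesh's relative Z from its starting height toward Distance, then replays after a delay.
; A timeline event track toggles CanKill, killing players already overlapping when it turns on, while the box's begin-overlap event catches those entering later.
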(event OnComponentBeginOverlap(Box)
  (params (OverlappedComponent :type Primitive%20Component%20Object%20Reference) (OtherActor :type Actor%20Object%20Reference) (OtherComp :type Primitive%20Component%20Object%20Reference) (OtherBodyIndex :type Integer) (bFromSweep :type Boolean) (SweepResult :type Hit%20Result%20Structure%20%28by%20ref%29))
  (bind _asbp_ia_player (Utilities|Casting|CastToBP_IA_Player OtherActor))
  (if (Variables|Default|GetCanKill)
    (Utilities|IsValid _asbp_ia_player
      (:Is%20Valid
        (Default|Death _asbp_ia_player)))))

(event Custom|Begin_TM
  (bind _staticmesh (Variables|Default|GetStaticMesh))
  (bind _relativelocation (Variables|/Script/Engine.SceneComponent|GetRelativeLocation _staticmesh))
  ;[1 1 1] Movement
  (bind _movement (Timeline|Timeline_0 PlayFromStart)
    (:Update
      (Transformation|SetRelativeLocation _staticmesh (Math|Vector|MakeVector (.x _relativelocation) (.y _relativelocation) (Math|Float|Lerp (Variables|Default|GetLocationZ) (Variables|Default|GetDistance) _movement)) false false))
    (:Finished
      (Utilities|FlowControl|Delay (Variables|Default|GetDelay))
      (CallFunction|BeginTM))
    (:CanKill
      (bind _output_get (Variables|Default|SetCanKill (not (Variables|Default|GetCanKill))))
      (if _output_get
        (CallFunction|Checkbox)))))

(event Custom|Checkbox
  (for _array_element (Collision|GetOverlappingActors (Variables|Default|GetBox) "/Game/Blueprints/Player/BP_IA_Player.BP_IA_Player_C" :!class /Script/Engine.PrimitiveComponent)
    (Utilities|IsValid _array_element
      (:Is%20Valid
        (bind _asbp_ia_player (Utilities|Casting|CastToBP_IA_Player _array_element))
        (Default|Death _asbp_ia_player)))))

(event EventBeginPlay
  ;[1 1 1] Initialisation
  (Components|Timeline|SetPlayRate (Variables|Default|GetTimeline_0) (Variables|Default|GetPlayRate))
  (Variables|Default|SetLocationZ (.z (Variables|/Script/Engine.SceneComponent|GetRelativeLocation (Variables|Default|GetStaticMesh))))
  (CallFunction|BeginTM))

(fn ConstructionScript
  (|CallParentFunction))