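; Moving wall trap that kills the player on contact while its CanKill flag is set.
; A timeline with configurable play rate lerps the mesh's relative X between zero and Distance, then restarts after a delay, looping from BeginPlay.
; Mesh overlap casts to BP_IA_Player and calls Death.
; A rotation timeline and a CanKill toggle are present but never run.
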(event OnComponentBeginOverlap(StaticMesh)
  (params (OverlappedComponent :type Primitive%20Component%20Object%20Reference) (OtherActor :type Actor%20Object%20Reference) (OtherComp :type Primitive%20Component%20Object%20Reference) (OtherBodyIndex :type Integer) (bFromSweep :type Boolean) (SweepResult :type Hit%20Result%20Structure%20%28by%20ref%29))
  ;[1 1 1] Hit (Death)
  (bind _asbp_ia_player (Utilities|Casting|CastToBP_IA_Player OtherActor))
  (if (Variables|Default|GetCanKill)
    (Utilities|IsValid _asbp_ia_player
      (:Is%20Valid
        (Default|Death _asbp_ia_player)))))

(event Custom|Begin_TM
  (bind _staticmesh (Variables|Default|GetStaticMesh))
  (bind _relativelocation (Variables|/Script/Engine.SceneComponent|GetRelativeLocation _staticmesh))
  ;[1 1 1] Movement
  (bind _movement (Timeline|Movement PlayFromStart)
    (:Update
      (Transformation|SetRelativeLocation _staticmesh (Math|Vector|MakeVector (Math|Float|Lerp 0.0 (Variables|Default|GetDistance) _movement) (.y _relativelocation) (.z _relativelocation)) false false))
    (:Finished
      (Utilities|FlowControl|Delay (Variables|Default|GetDelay))
      (CallFunction|BeginTM))))

(event EventBeginPlay
  ;[1 1 1] Initialisation
  (Components|Timeline|SetPlayRate (Variables|Default|GetMovement) (Variables|Default|GetPlayRate))
  (CallFunction|BeginTM))

(fn ConstructionScript
  (|CallParentFunction))