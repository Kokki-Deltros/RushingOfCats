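; Finish line for a playground level, deciding win or loss once every cat in the player's group has crossed it.
; Each BP_IA_Player leaving FinishBox is counted once toward the player's NbOfCatsSuccessed.
; When all have crossed and the quota is met, the group loops a jump animation, surplus cats add to TempCoin and the completed screen shows.
; Otherwise the failed screen shows; both outcomes remove the player widget and halt player movement.
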(event OnComponentEndOverlap(FinishBox)
  (params (OverlappedComponent :type Primitive%20Component%20Object%20Reference) (OtherActor :type Actor%20Object%20Reference) (OtherComp :type Primitive%20Component%20Object%20Reference) (OtherBodyIndex :type Integer))
  (bind _returnvalue (Game|GetPlayerCharacter 0))
  (bind _asbp_movement_player (Utilities|Casting|CastToBP_Movement_Player _returnvalue))
  (bind _nb_of_cats_needed (Variables|/Game/Blueprints/Player/BP_Movement_Player.BP_Movement_Player_C|GetNb_Of_Cats_Needed _asbp_movement_player))
  (bind _nb_of_cats_successed (Variables|/Game/Blueprints/Player/BP_Movement_Player.BP_Movement_Player_C|GetNb_Of_Cats_Successed _asbp_movement_player))
  (bind _charactermovement (Variables|/Script/Engine.Character|GetCharacterMovement _asbp_movement_player))
  (bind _groupe (Variables|/Game/Blueprints/Player/BP_Movement_Player.BP_Movement_Player_C|GetGroupe _asbp_movement_player))
  (bind _charactermovement_2 (Variables|/Script/Engine.Character|GetCharacterMovement _asbp_movement_player))
  (bind _returnvalue_2 (Utilities|Array|Length _groupe))
  (bind _returnvalue_3 (== _nb_of_cats_successed _returnvalue_2))
  (bind _asbp_ia_player (Utilities|Casting|CastToBP_IA_Player OtherActor))
  (if (not (Variables|/Game/Blueprints/Player/BP_IA_Player.BP_IA_Player_C|GetAddedFinish _asbp_ia_player))
    (Variables|/Game/Blueprints/Player/BP_IA_Player.BP_IA_Player_C|SetAddedFinish _asbp_ia_player true)
    (Math|Integer|IncrementInt _nb_of_cats_successed
      (:%20%20
        (if (and (>= _nb_of_cats_successed _nb_of_cats_needed) _returnvalue_3)
          (for _array_element (Variables|/Game/Blueprints/Player/BP_Movement_Player.BP_Movement_Player_C|GetGroupe _asbp_movement_player)
            (Components|Animation|PlayAnimation (Variables|/Script/Engine.Character|GetMesh _array_element) "/Game/Animations/Player/Anim_Jump.Anim_Jump" true))
          (Variables|/Game/Blueprints/Player/BP_Movement_Player.BP_Movement_Player_C|SetFinish _asbp_movement_player true)
          (Utilities|FlowControl|Delay 1.5)
          (Variables|/Game/Blueprints/Player/BP_Movement_Player.BP_Movement_Player_C|SetTemp_Coin _asbp_movement_player (+ (Variables|/Game/Blueprints/Player/BP_Movement_Player.BP_Movement_Player_C|GetTemp_Coin _asbp_movement_player) (- _nb_of_cats_successed _nb_of_cats_needed)))
          (Widget|RemovefromParent (Variables|/Game/Blueprints/Player/BP_Movement_Player.BP_Movement_Player_C|GetWG_Player_Ref _asbp_movement_player))
          (bind _returnvalue_4 (UserInterface|CreateWidget "/Game/Blueprints/Widget/WG_Level_Completed.WG_Level_Completed_C"))
          (UserInterface|Viewport|AddtoViewport _returnvalue_4 0)
          (Components|Movement|StopMovementImmediately _charactermovement_2)
          (Variables|/Script/Engine.CharacterMovementComponent|SetMaxWalkSpeed _charactermovement_2 0.0)
          (elif _returnvalue_3
            (Utilities|FlowControl|Delay 1.5)
            (Widget|RemovefromParent (Variables|/Game/Blueprints/Player/BP_Movement_Player.BP_Movement_Player_C|GetWG_Player_Ref _asbp_movement_player))
            (Variables|/Game/Blueprints/Player/BP_Movement_Player.BP_Movement_Player_C|SetFinish _asbp_movement_player true)
            (Variables|/Game/Blueprints/Player/BP_Movement_Player.BP_Movement_Player_C|SetLose _asbp_movement_player true)
            (bind _returnvalue_5 (UserInterface|CreateWidget "/Game/Blueprints/Widget/WG_Level_Failed.WG_Level_Failed_C"))
            (bind _output_get (Variables|Default|SetWG_Level_Failed _returnvalue_5))
            (UserInterface|Viewport|AddtoViewport _output_get 0)
            (Components|Movement|StopMovementImmediately (Variables|/Script/Engine.Character|GetCharacterMovement _asbp_movement_player))
            (Variables|/Script/Engine.CharacterMovementComponent|SetMaxWalkSpeed (Variables|/Script/Engine.Character|GetCharacterMovement _asbp_ia_player) 0.0)
            (Components|Movement|StopMovementImmediately _charactermovement)
            (Variables|/Script/Engine.CharacterMovementComponent|SetMaxWalkSpeed _charactermovement 0.0)))))))

(fn ConstructionScript)