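; BP_MultiCoin is a pickup that awards three coins when a BP_IA_Player overlaps it.
; If that character is active, it plays one of two random coin sounds and adds the coins to the TempCoin count on its RefPlayer.
; It then shows a WG_NbOfGoldTook widget with the amount gained and destroys itself.
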(event Collision|EventActorBeginOverlap
  (params (OtherActor :type Actor%20Object%20Reference))
  (bind _asbp_ia_player (Utilities|Casting|CastToBP_IA_Player OtherActor))
  (Utilities|IsValid self
    (:Is%20Valid
      (if (Variables|/Game/Blueprints/Player/BP_IA_Player.BP_IA_Player_C|GetIsActive _asbp_ia_player)
        (Audio|PlaySound2D (Utilities|Select :Index (Math|Random|RandomIntegerinRange 0 1) :Option%200 "/Game/Sounds/SFX/Coin1_Cue.Coin1_Cue" :Option%201 "/Game/Sounds/SFX/Coin2_Cue.Coin2_Cue") 1.0 1.0 0.0 0 0)
        (Variables|/Game/Blueprints/Player/BP_Movement_Player.BP_Movement_Player_C|SetTemp_Coin (Variables|/Game/Blueprints/Player/BP_IA_Player.BP_IA_Player_C|GetRef%20Player _asbp_ia_player) (+ (Variables|/Game/Blueprints/Player/BP_Movement_Player.BP_Movement_Player_C|GetTemp_Coin (Variables|/Game/Blueprints/Player/BP_IA_Player.BP_IA_Player_C|GetRef%20Player _asbp_ia_player)) 3))
        (bind _returnvalue (UserInterface|CreateWidget "/Game/Blueprints/Widget/Pop_Up/WG_+NbOfGoldTook.WG_+NbOfGoldTook_C" 0 3))
        (UserInterface|Viewport|AddtoViewport _returnvalue 0)
        (Actor|DestroyActor :!label _label)))
    (:Is%20Not%20Valid
      (goto _label))))

(fn ConstructionScript)