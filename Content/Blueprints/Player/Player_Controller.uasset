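; Player controller that owns save and load of the player's progress through a single TheSaveGame slot.
; On BeginPlay it async-loads the slot and copies level, skins, coins, max platform count and cats needed onto BP_Movement_Player, or creates a fresh save object if none exists.
; The SaveGame event packs those same character values back into the save struct and writes the slot.
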(event Custom|Save%20Game
  (bind _returnvalue (Game|GetPlayerCharacter 0))
  (bind _asbp_movement_player (Utilities|Casting|CastToBP_Movement_Player _returnvalue))
  ;[1 1 1] Save Game
  (Variables|/Game/Blueprints/Save/TheSaveGame.TheSaveGame_C|SetStruct_Save_Save (Variables|Default|GetTheSaveGame_Ref) (Utilities|Struct|MakeStruct_Save (Variables|/Game/Blueprints/Player/BP_Movement_Player.BP_Movement_Player_C|GetCurrent_Level _asbp_movement_player) (Variables|/Game/Blueprints/Player/BP_Movement_Player.BP_Movement_Player_C|GetSkin _asbp_movement_player) (Variables|/Game/Blueprints/Player/BP_Movement_Player.BP_Movement_Player_C|GetCoin _asbp_movement_player) (Variables|/Game/Blueprints/Player/BP_Movement_Player.BP_Movement_Player_C|GetStruct_Skin_Player _asbp_movement_player) (Variables|/Game/Blueprints/Player/BP_Movement_Player.BP_Movement_Player_C|GetMax_Nb_Platform _asbp_movement_player) (Variables|/Game/Blueprints/Player/BP_Movement_Player.BP_Movement_Player_C|GetNb_Of_Cats_Needed _asbp_movement_player)))
  (SaveGame|SaveGametoSlot (Variables|Default|GetTheSaveGame_Ref) "TheSaveGame"))

(event Custom|Load%20Game
  (bind _returnvalue (Game|GetPlayerCharacter 0))
  (bind _asbp_movement_player (Utilities|Casting|CastToBP_Movement_Player _returnvalue))
  ;[1 1 1] Load Game
  (bind _returnvalue_2 (SaveGame|DoesSaveGameExist "TheSaveGame"))
  (if _returnvalue_2
    (bind _savegame (|AsyncLoadGamefromSlot "TheSaveGame")
      (:Completed
        (bind _asthe_save_game (Utilities|Casting|CastToTheSaveGame _savegame))
        (bind _output_get (Variables|Default|SetTheSaveGame_Ref _asthe_save_game))
        (Variables|/Game/Blueprints/Player/BP_Movement_Player.BP_Movement_Player_C|SetCurrent_Level _asbp_movement_player (.level (Variables|/Game/Blueprints/Save/TheSaveGame.TheSaveGame_C|GetStruct_Save_Save _output_get)))
        (Variables|/Game/Blueprints/Player/BP_Movement_Player.BP_Movement_Player_C|SetSkin _asbp_movement_player (.skin (Variables|/Game/Blueprints/Save/TheSaveGame.TheSaveGame_C|GetStruct_Save_Save _output_get)))
        (Variables|/Game/Blueprints/Player/BP_Movement_Player.BP_Movement_Player_C|SetCoin _asbp_movement_player (.coin (Variables|/Game/Blueprints/Save/TheSaveGame.TheSaveGame_C|GetStruct_Save_Save _output_get)))
        (Variables|/Game/Blueprints/Player/BP_Movement_Player.BP_Movement_Player_C|SetMax_Nb_Platform _asbp_movement_player (.maxnbplateform (Variables|/Game/Blueprints/Save/TheSaveGame.TheSaveGame_C|GetStruct_Save_Save _output_get)))
        (Variables|/Game/Blueprints/Player/BP_Movement_Player.BP_Movement_Player_C|SetStruct_Skin_Player _asbp_movement_player (.structskinsplayer (Variables|/Game/Blueprints/Save/TheSaveGame.TheSaveGame_C|GetStruct_Save_Save _output_get)))
        (Variables|/Game/Blueprints/Player/BP_Movement_Player.BP_Movement_Player_C|SetNb_Of_Cats_Needed _asbp_movement_player (.catsneeded (Variables|/Game/Blueprints/Save/TheSaveGame.TheSaveGame_C|GetStruct_Save_Save _output_get)))))
    (else
      (CallFunction|NewGame))))

(event Custom|New%20Game
  ;[1 1 1] New Game
  (bind _returnvalue (SaveGame|CreateSaveGameObject "/Game/Blueprints/Save/TheSaveGame.TheSaveGame_C"))
  (Variables|Default|SetTheSaveGame_Ref _returnvalue))

(event EventBeginPlay
  (CallFunction|LoadGame))

(fn ConstructionScript)